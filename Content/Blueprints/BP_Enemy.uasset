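; BP_Enemy is a simple enemy actor that announces itself on BeginPlay and can take damage until it dies.
; A TakeDamage event subtracts the incoming amount from Health and prints a damage message.
; The CheckIfAlive function tests whether Health is above zero; when it is not, the actor prints a death message and destroys itself.
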(event Custom|Take%20Damage
  (params (By :type Float%20%28double-precision%29))
  (Variables|Default|SetHealth (- (Variables|Default|GetHealth) By))
  (Development|PrintString (Utilities|String|Append "Ouch! My health is now " (Utilities|String|ToString(Float) (- (Variables|Default|GetHealth) By))) true true "(R=0.475000,G=0.000000,B=0.042399,A=1.000000)")
  (bind _isalive (CallFunction|CheckifAlive (Variables|Default|GetHealth)))
  (if (not _isalive)
    (Development|PrintString "Man I'm dead!")
    (Actor|DestroyActor)))

(event EventBeginPlay
  (Development|PrintString "Hello, I have been programmed to destroy you!"))

(event Collision|EventActorBeginOverlap
  (params (OtherActor :type Actor%20Object%20Reference)))

(event EventTick
  (params (DeltaSeconds :type Float%20%28single-precision%29)))

(fn ConstructionScript)

(fn CheckifAlive
  (params (Health :type Float%20%28double-precision%29))
  (return (> Health 0.0)))