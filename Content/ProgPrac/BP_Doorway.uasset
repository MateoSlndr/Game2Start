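; BP_Doorway is a doorway trigger, apparently for programming practice, that prints a debug message based on its DoorType when the player character class walks into it.
; BoxCollision's begin overlap casts the other actor to BP_ThirdPersonCharacter, then switches on DoorType, with a fallback message for unhandled values.
; An unconnected nested-branch version of the same selection remains in the graph and never runs.
; No door movement or other gameplay effect is implemented.
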(event OnComponentBeginOverlap(BoxCollision)
  (params (OverlappedComponent :type Primitive%20Component%20Object%20Reference) (OtherActor :type Actor%20Object%20Reference) (OtherComp :type Primitive%20Component%20Object%20Reference) (OtherBodyIndex :type Integer) (bFromSweep :type Boolean) (SweepResult :type Hit%20Result%20Structure%20%28by%20ref%29))
  (Utilities|Casting|CastToBP_ThirdPersonCharacter OtherActor)
  (switch int (Variables|Default|GetDoorType)
    (:Default
      (Development|PrintString "WTF"))
    (:0
      (Development|PrintString "Zero is a weird number"))
    (:1
      (Development|PrintString "One is the loneliest number"))
    (:2
      (Development|PrintString "Two is trouble"))))

(event EventBeginPlay)

(event Collision|EventActorBeginOverlap
  (params (OtherActor :type Actor%20Object%20Reference)))

(event EventTick
  (params (DeltaSeconds :type Float%20%28single-precision%29)))

(fn ConstructionScript)