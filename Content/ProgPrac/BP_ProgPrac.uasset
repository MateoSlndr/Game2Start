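; BP_ProgPrac is an actor, apparently for programming practice, that endlessly spawns random pickups around its location.
; On BeginPlay it draws a debug circle of its Radius, randomly may set HasKey, and prints score, health, player name and key state.
; SpawnPickup calls itself after a fixed delay, spawning a random Pickups class within that radius by flattening a scaled random unit vector onto the horizontal plane.
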(event Custom|Spawn%20Pickup
  (bind _radius (Variables|Default|GetRadius))
  (bind _pickups (Variables|Default|GetPickups))
  (Utilities|FlowControl|Delay 1.7)
  (Game|SpawnActorfromClass (Utilities|Array|Get(acopy) _pickups (Math|Random|RandomIntegerinRange 0 (- (Utilities|Array|Length _pickups) 1))) (Math|Transform|MakeTransform (+ (Transformation|GetWorldLocation (Variables|Default|GetDefaultSceneRoot)) (* (Math|Random|RandomUnitVector) (Math|Vector|MakeVector _radius _radius 0.0))) "0, 0, 0" "1.000000,1.000000,1.000000") "Undefined" "MultiplyWithRoot" 0 0)
  (CallFunction|SpawnPickup))

(event EventBeginPlay
  (Rendering|Debug|DrawDebugCircle (Transformation|GetWorldLocation (Variables|Default|GetDefaultSceneRoot)) (Variables|Default|GetRadius) 64 "(R=1.000000,G=1.000000,B=1.000000,A=1.000000)" 6e+01 1e+01 "0.000000,1.000000,0.000000" "1.000000,0.000000,0.000000" true)
  (if (> (Math|Random|RandomFloat) 0.5)
    (Variables|Default|SetHasKey true))
  (Development|PrintString (Utilities|String|Append " Score" (Utilities|String|ToString(Integer) (Variables|Default|GetScore)) " Health" (Utilities|String|ToString(Float) (Variables|Default|GetHealth)) " PlayerName" (Variables|Default|GetPlayerName) " HasKey" (Utilities|String|ToString(Boolean) (Variables|Default|GetHasKey))) true true "(R=0.000000,G=0.660000,B=1.000000,A=1.000000)" 5.0)
  (CallFunction|SpawnPickup))

(event Collision|EventActorBeginOverlap
  (params (OtherActor :type Actor%20Object%20Reference)))

(event EventTick
  (params (DeltaSeconds :type Float%20%28single-precision%29)))

(fn ConstructionScript)